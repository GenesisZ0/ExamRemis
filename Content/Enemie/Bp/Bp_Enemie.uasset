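; Enemy Blueprint that tracks health in PV and handles getting hit and dying.
; TakeDamage subtracts damage from PV, plays the hit animation on the mesh, and calls Die once PV reaches zero or below.
; Die plays the death animation directly on the mesh, waits briefly, then destroys the actor.
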(event `TakeDamage`
  (params (Damage :type "Float (double-precision)"))
  (set `self.PV` (- (`self.PV`) Damage))
  (`SkeletalMeshComponent.PlayAnimation` (`self.Mesh`) "/Game/GetHitAnim.GetHitAnim" false)
  (if (<= (`self.PV`) 0.0)
    (`self.Die`)))

(event `Die`
  (`SkeletalMeshComponent.PlayAnimation` (`self.Mesh`) "/Game/DieAnim.DieAnim" false)
  (`KismetSystemLibrary.Delay` 2.0)
  (`self.K2_DestroyActor`))

(fn `UserConstructionScript`)